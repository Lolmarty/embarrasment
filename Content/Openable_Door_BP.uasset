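; Openable door actor that swings open and closed in response to requests from its OpenDoor component or interface.
; It stores its starting rotation on BeginPlay, then a timeline drives a yaw offset combined with that rotation.
; Close requests reverse the same timeline, and an event track on it plays the door lock sound at the actor's location.
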(event OnOpenRequest(OpenDoor)
  (bind _swing (Timeline|Timeline_0 Play)
    (:Update
      (Transformation|SetActorRotation (Math|Rotator|CombineRotators (Variables|Default|GetInitialRotation) (Math|Rotator|MakeRotator 0.0 0.0 _swing))))
    (:AudioCurve
      (Audio|PlaySoundatLocation "/Game/UserSounds/door-lock.door-lock" (Transformation|GetActorLocation) "0, 0, 0" 1.0 1.0 0.0 0 0 0))))

(event OnCloseRequest(OpenDoor)
  (bind _swing (Timeline|Timeline_0 Reverse)
    (:Update
      (Transformation|SetActorRotation (Math|Rotator|CombineRotators (Variables|Default|GetInitialRotation) (Math|Rotator|MakeRotator 0.0 0.0 _swing))))
    (:AudioCurve
      (Audio|PlaySoundatLocation "/Game/UserSounds/door-lock.door-lock" (Transformation|GetActorLocation) "0, 0, 0" 1.0 1.0 0.0 0 0 0))))

(event EventBeginPlay
  (Variables|Default|SetInitialRotation (Transformation|GetActorRotation)))

(fn ConstructionScript)